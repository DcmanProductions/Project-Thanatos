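; Utility Blueprint of shared helpers for book lookup, player access, value inversion, UI facing and joystick direction.
; GetBook returns an indexed or random book, though the random range excludes the last entry.
; UI rotation yaws a widget toward player zero using a flattened target-to-player vector, while GetOppositeScaledValue reduces to maximum minus current.
; GetJoystickDirection branches by stick but has only constant zero inputs, so always returns a zero vector.
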(fn GetBook
  (params (IsRandom :type Boolean) (Index :type Integer))
  (bind _books (LocalVariables|GetBooks))
  (return (Utilities|Array|Get(acopy) _books (Math|Integer|SelectInt (Math|Random|RandomInteger (- (Utilities|Array|Length _books) 1)) Index IsRandom))))

(fn GetPlayer
  (params (Index :type Integer))
  (return (.AsPlayer (Utilities|Casting|CastToPlayer (Game|GetPlayerCharacter 0 Index)))))

(fn GetOppositeScaledValue
  (params (Max%20Scaled%20Value :type Float%20%28single-precision%29) (Current%20Scaled%20Value :type Float%20%28single-precision%29))
  (return (- Current%20Scaled%20Value (- (/ Current%20Scaled%20Value 0.5) Max%20Scaled%20Value))))

(fn UpdateUIRotationtoMeetPlayerGaze
  (params (Target :type Actor%20Object%20Reference) (Widget :type Scene%20Component%20Object%20Reference))
  (bind _player (CallFunction|GetPlayer))
  (Utilities|IsValid Widget
    (:Is%20Valid
      (Utilities|IsValid _player
        (:Is%20Valid
          (Transformation|SetWorldRotation Widget (Math|Conversions|RotationFromXVector (Math|Vector|RotateVector (Math|Vector|Normalize (* (- (Transformation|GetActorLocation _player) (Transformation|GetActorLocation Target)) "1.000000,1.000000,0.000000")) "0, 0, 0")) false false))))))

(fn GetJoystickDirection
  (params (Stick :type EJoystickTypes%20Enum :default "NewEnumerator0"))
  (switch Utilities|FlowControl|Switch|SwitchonEJoystickTypes Stick
    (:NewEnumerator0
      (return (Math|Vector2D|MakeVector2D 0.0 (* 0.0 -1.0))))
    (:NewEnumerator1
      (return (Math|Vector2D|MakeVector2D 0.0 0.0)))))