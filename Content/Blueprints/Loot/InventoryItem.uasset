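; Loot pickup actor that the player equips as a weapon on interact, then hides and destroys.
; On BeginPlay it fills its info widget with a title and detail rows, including weight, and each Tick turns it toward the player's gaze.
; An overlap range starts a self-repeating, delayed camera line trace against the mesh and widget, which updates CanInteract and the player's current loot target.
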(event OnComponentBeginOverlap(InteractionRange)
  (params (OverlappedComponent :type Primitive%20Component%20Object%20Reference) (OtherActor :type Actor%20Object%20Reference) (OtherComp :type Primitive%20Component%20Object%20Reference) (OtherBodyIndex :type Integer) (bFromSweep :type Boolean) (SweepResult :type Hit%20Result%20Structure%20%28by%20ref%29))
  ;[0 1 0.2662] Sets when player is in range to interact
  (bind _asplayer (Utilities|Casting|CastToPlayer OtherActor))
  (Variables|Default|SetInRange true)
  (Variables|/Game/Blueprints/Entities/Player/Player.Player_C|SetCurrentInteractObject _asplayer 0)
  (CallFunction|Find (Variables|/Game/Blueprints/Entities/Player/Player.Player_C|GetFollowCamera _asplayer)))

(event OnComponentEndOverlap(InteractionRange)
  (params (OverlappedComponent :type Primitive%20Component%20Object%20Reference) (OtherActor :type Actor%20Object%20Reference) (OtherComp :type Primitive%20Component%20Object%20Reference) (OtherBodyIndex :type Integer))
  ;[1 0.03535 0] Sets when player is NOT in range to interact
  (bind _asplayer (Utilities|Casting|CastToPlayer OtherActor))
  (Variables|Default|SetInRange false)
  (Variables|/Game/Blueprints/Entities/Player/Player.Player_C|SetCurrentInteractObject _asplayer 0))

(event Custom|Interact
  ;[0 0.4839 1] Interact
  (if (Variables|Default|GetCanInteract)
    (Default|EquiptWeapon (CallFunction|GetPlayer) self)
    (Rendering|SetVisibility (Variables|Default|Get%20MeshObject) false true)
    (Actor|DestroyActor)))

(event Custom|Find
  (params (From :type Scene%20Component%20Object%20Reference))
  (bind _returnvalue (Transformation|GetWorldLocation From))
  (bind _player (CallFunction|GetPlayer))
  ;[1 0.115 0.7365] Checks if Player is looking at an Interactable Object
  (if (Variables|Default|GetInRange)
    (bind _outhit (Collision|LineTraceByChannel _returnvalue (+ _returnvalue (* (Math|Vector|GetForwardVector (Transformation|GetWorldRotation From)) 300)) "TraceTypeQuery1" false 0 "None" false))
    (if (or (== (.HitComponent (Collision|BreakHitResult _outhit)) (Variables|Default|Get%20MeshObject)) (== (.HitComponent (Collision|BreakHitResult _outhit)) (Variables|Default|GetItemInformation)))
      (Utilities|FlowControl|Delay 0.2 :!label _label)
      (Variables|Default|SetCanInteract true)
      (Variables|/Game/Blueprints/Entities/Player/Player.Player_C|SetCurrentInteractLootObject _player self)
      (CallFunction|Find From)
      (else
        (Utilities|FlowControl|Sequence
          (:then_0
            (Variables|Default|SetCanInteract false :!label _label_2)
            (Variables|/Game/Blueprints/Entities/Player/Player.Player_C|SetCurrentInteractLootObject _player 0))
          (:then_1
            (goto _label)))))
    (else
      (goto _label_2))))

(event EventBeginPlay
  ;[0 1 0.08333] Begin Play
  (Utilities|FlowControl|Sequence
    (:then_0
      ;;[1 1 1] Add Default Items
      (Utilities|Array|Add (Variables|InventoryItem|GetItemDetails) (Utilities|Struct|MakeStruct_LootItemDescription "Weight" (Utilities|Text|ToText(Float) (Variables|InventoryItem|GetWeight) "HalfToEven"))))
    (:then_1
      ;;[0 0.2833 1] Adding Loot Item Description
      (bind _asloot_intormation (Utilities|Casting|CastToLootIntormation (UserInterface|GetWidget (Variables|Default|GetItemInformation))))
      (bind _output_get (Variables|Default|SetLoot%20Intormation%20Widget _asloot_intormation))
      (for _array_element (Variables|InventoryItem|GetItemDetails)
        (bind _returnvalue (UserInterface|CreateWidget "/Game/Blueprints/UI/Loot/LootInformationDetail.LootInformationDetail_C"))
        (Utilities|IsValid _returnvalue
          (:Is%20Valid
            (Utilities|FlowControl|Sequence
              (:then_0
                (Variables|/Game/Blueprints/UI/Loot/LootInformationDetail.LootInformationDetail_C|SetDetailItemTitle _returnvalue (.lootitemtitle _array_element)))
              (:then_1
                (Variables|/Game/Blueprints/UI/Loot/LootInformationDetail.LootInformationDetail_C|SetDetailItemValue _returnvalue (.lootitemvalue _array_element)))
              (:then_2
                (Utilities|Array|Add (Variables|/Game/Blueprints/UI/Loot/LootIntormation.LootIntormation_C|GetLootDetails _output_get) _returnvalue)))))))
    (:then_2
      ;;[1 1 1] Set Item Title
      (Variables|/Game/Blueprints/UI/Loot/LootIntormation.LootIntormation_C|SetItemTitle (Variables|Default|GetLoot%20Intormation%20Widget) (Variables|InventoryItem|GetItemTitle)))))

(event EventTick
  (params (DeltaSeconds :type Float%20%28single-precision%29))
  ;[1 1 1] Tick
  (CallFunction|UpdateUIRotationtoMeetPlayerGaze self (Variables|Default|GetItemInformation)))

(fn ConstructionScript)